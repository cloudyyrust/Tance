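; Interactable world item that shows proximity icons to the player and destroys itself when used.
; Outer and inner spheres, sized in the construction script, toggle the far and near icons on player overlap.
; Tick polls the first-person character's IsInteracting and HitActor, firing Interacted, which prints and destroys after a short delay.
; A separate Interact function destroys the item immediately and returns false.
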(event OnComponentBeginOverlap(InnerSphereCollsion)
  (params (OverlappedComponent :type Primitive%20Component%20Object%20Reference) (OtherActor :type Actor%20Object%20Reference) (OtherComp :type Primitive%20Component%20Object%20Reference) (OtherBodyIndex :type Integer) (bFromSweep :type Boolean) (SweepResult :type Hit%20Result%20Structure%20%28by%20ref%29))
  (if (== OtherActor (Game|GetPlayerCharacter 0))
    (Rendering|SetVisibility (Variables|Default|GetInnerinteracticon) true false)
    (Rendering|SetVisibility (Variables|Default|GetOuterinteracticon) false false)))

(event OnComponentEndOverlap(InnerSphereCollsion)
  (params (OverlappedComponent :type Primitive%20Component%20Object%20Reference) (OtherActor :type Actor%20Object%20Reference) (OtherComp :type Primitive%20Component%20Object%20Reference) (OtherBodyIndex :type Integer))
  (if (== (Game|GetPlayerCharacter 0) OtherActor)
    (Rendering|SetVisibility (Variables|Default|GetInnerinteracticon) false false)
    (Rendering|SetVisibility (Variables|Default|GetOuterinteracticon) true false)))

(event OnComponentBeginOverlap(OuterSpherecollsion)
  (params (OverlappedComponent :type Primitive%20Component%20Object%20Reference) (OtherActor :type Actor%20Object%20Reference) (OtherComp :type Primitive%20Component%20Object%20Reference) (OtherBodyIndex :type Integer) (bFromSweep :type Boolean) (SweepResult :type Hit%20Result%20Structure%20%28by%20ref%29))
  (if (== OtherActor (Game|GetPlayerCharacter 0))
    (Rendering|SetVisibility (Variables|Default|GetOuterinteracticon) true false)))

(event OnComponentEndOverlap(OuterSpherecollsion)
  (params (OverlappedComponent :type Primitive%20Component%20Object%20Reference) (OtherActor :type Actor%20Object%20Reference) (OtherComp :type Primitive%20Component%20Object%20Reference) (OtherBodyIndex :type Integer))
  (if (== (Game|GetPlayerCharacter 0) OtherActor)
    (Rendering|SetVisibility (Variables|Default|GetOuterinteracticon) false false)))

(event Custom|Interacted
  (Development|PrintString "Interacted")
  (Utilities|FlowControl|Delay 0.5)
  (Actor|DestroyActor))

(event EventBeginPlay
  (bind _asbp_first_person_character (Utilities|Casting|CastToBP_FirstPersonCharacter (Game|GetPlayerCharacter 0)))
  (Variables|Default|SetBP_Player%20Ref _asbp_first_person_character))

(event EventTick
  (params (DeltaSeconds :type Float%20%28single-precision%29))
  (bind _bp_player_ref (Variables|Default|GetBP_Player%20Ref))
  (if (and (Variables|/Game/FirstPerson/Blueprints/BP_FirstPersonCharacter.BP_FirstPersonCharacter_C|GetIs%20Interacting? _bp_player_ref) (== (Variables|/Game/FirstPerson/Blueprints/BP_FirstPersonCharacter.BP_FirstPersonCharacter_C|GetHit%20Actor _bp_player_ref) self))
    (CallFunction|Interacted)))

(fn ConstructionScript
  (Components|Sphere|SetSphereRadius (Variables|Default|GetInnerSphereCollsion) (Variables|Public|GetInnerSphereRadius) true)
  (Components|Sphere|SetSphereRadius (Variables|Default|GetOuterSpherecollsion) (Variables|Public|GetouterSphereRadius) true))

(fn Interact
  (params (Interactor%20 :type Character%20Object%20Reference))
  (Actor|DestroyActor)
  (return false))