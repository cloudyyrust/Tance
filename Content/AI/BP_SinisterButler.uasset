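; Sinister Butler AI pawn that pursues the player and has physics-simulated chains on its skeletal mesh.
; FollowPlayer runs AI MoveTo on the player character, printing debug text and calling itself two seconds after each success; failure has no handler.
; Nothing in this graph calls FollowPlayer, as BeginPlay is empty.
; Tick re-enables physics simulation below each bone named in Chains every frame.
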(event Custom|FollowPlayer
  (Development|PrintString "AI" true true "(R=1.000000,G=0.000000,B=0.167367,A=1.000000)")
  (AI|AIMoveTo self "0, 0, 0" (Game|GetPlayerCharacter 0) 5.0 false
    (:OnSuccess
      (Development|PrintString "AI Hunt Sucess" true true "(R=0.000000,G=1.000000,B=0.138429,A=1.000000)")
      (Utilities|FlowControl|Delay 2.0)
      (CallFunction|FollowPlayer))))

(event EventBeginPlay)

(event EventTick
  (params (DeltaSeconds :type Float%20%28single-precision%29))
  (for _array_element (Variables|Default|GetChains)
    (Class|SkeletalMeshComponent|SetAllBodiesBelowSimulatePhysics (Variables|Character|GetMesh) _array_element true true)))

(fn ConstructionScript)